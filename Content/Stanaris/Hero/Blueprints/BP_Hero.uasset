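; Player hero Blueprint that toggles the inventory UI and picks up world items.
; Tab or B shows or hides the WHero widget, obtained through the hero controller's layout, along with the mouse cursor.
; E traces from the follow camera for a BP_BaseItem, whose data BPInventoryComp fits into empty slots by icon size and template indexes.
; A fitting item fills every covered slot, leaves the world and gets an inventory widget slot; otherwise a full-inventory message prints.
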(event `self.ReceiveBeginPlay`
  (bind _asbp_hero_controller (cast `/Game/Stanaris/Hero/Blueprints/BP_HeroController` (`GameplayStatics.GetPlayerController` 0)))
  (bind _output_get (set `self.ControllerRef` _asbp_hero_controller))
  (set `self.W_HeroRef` (`/Game/Stanaris/Hero/UI/W_Layout.W_Hero` (`/Game/Stanaris/Hero/Blueprints/BP_HeroController.W_LayoutRef` _output_get))))

(event `Key|Tab`
  (params (Key :type "Key Structure"))
  (bind _w_heroref (`self.W_HeroRef`))
  (bind _controllerref (`self.ControllerRef`))
  ;[1 1 1] Open inventory
  (:`Pressed`
    (if (`Widget.IsVisible` (`self.W_HeroRef`)) :!label _label
      (`Widget.SetVisibility` _w_heroref "Hidden")
      (set `PlayerController.bShowMouseCursor` false _controllerref)
      (else
        (`Widget.SetVisibility` _w_heroref "SelfHitTestInvisible")
        (set `PlayerController.bShowMouseCursor` true _controllerref)))))

(event `Key|B`
  (params (Key :type "Key Structure"))
  ;[1 1 1] Open inventory
  (:`Pressed`
    (goto _label)))

(event `Key|E`
  (params (Key :type "Key Structure"))
  (bind _followcamera (`self.FollowCamera`))
  (bind _returnvalue (`SceneComponent.K2_GetComponentLocation` _followcamera))
  (:`Pressed`
    (bind (_outhit _returnvalue_2) (`KismetSystemLibrary.LineTraceSingle` :`Start` _returnvalue :`End` (+ _returnvalue (* (`SceneComponent.GetForwardVector` _followcamera) 200.0)) :`TraceChannel` "TraceTypeQuery1" :`DrawDebugType` "ForDuration"))
    (if _returnvalue_2
      (bind (_bblockinghit _binitialoverlap _time _distance _location _impactpoint _normal _impactnormal _physmat _hitactor) (`GameplayStatics.BreakHitResult` _outhit))
      (cast `/Game/Stanaris/Blueprints/BP_BaseItem` _hitactor)
      (bind _dataitem (message `/Game/Stanaris/Hero/Blueprints/Interface/BPI_TouchItem.TouchItem` _hitactor))
      (bind ((`IconSize` _iconsize) (`TemplateIndexes` _templateindexes)) (break `DataItems` _dataitem))
      (bind (_found _emptyslotsindex) (`/Game/Stanaris/Hero/Blueprints/Components/BP_InventoryComp.FindEmptySlot` (`self.BP_InventoryComp`) _iconsize _templateindexes))
      (if _found
        (for _array_element _emptyslotsindex
          (`KismetArrayLibrary.Array_Set` (`/Game/Stanaris/Hero/Blueprints/Components/BP_InventoryComp.StoreItems` (`self.BP_InventoryComp`)) _array_element _dataitem))
        (`self.K2_DestroyActor` _hitactor)
        (`/Game/Stanaris/Hero/Blueprints/Components/BP_InventoryComp.CreateItemSlotToInventory` (`self.BP_InventoryComp`) _emptyslotsindex _dataitem)
        (else
          (`KismetSystemLibrary.PrintString` "inventory is full"))))))

(fn `TouchItem`)

(fn `UserConstructionScript`)