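; Hero inventory component that stores items in a fixed grid where one item can span several slots.
; The grid is a flat StoreItems array sized XSlots by YSlots, with Id -1 marking a free slot.
; FindEmptySlot scans for a position where all template index offsets fit via CanItemToSlots, and PlaceItemToStore fills those indexes.
; CreateItemSlotToInventory adds a W_ItemSlot to the HUD grid, spanned to the icon size.
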(event `self.ReceiveBeginPlay`
  (`self.InitInventory`)
  (bind _asbp_hero_controller (cast `/Game/Stanaris/Hero/Blueprints/BP_HeroController` (`GameplayStatics.GetPlayerController` 0)))
  (bind _output_get (set `self.ControllerRef` _asbp_hero_controller))
  (set `self.W_InventoryRef` (`/Game/Stanaris/Hero/UI/W_Hero.W_Inventory` (`/Game/Stanaris/Hero/UI/W_Layout.W_Hero` (`/Game/Stanaris/Hero/Blueprints/BP_HeroController.W_LayoutRef` _output_get)))))

(fn `CanItemToSlots`
  (params (ToSlot :type Integer) (TemplateIndexes :type "Array of Integer"))
  (returns (IsFounded :type Boolean) (EmptySlotsIndexes :type "Array of Integer"))
  (locals (L_TemplateIndexes :type "Array of Integer") (L_StoreIndex :type Integer) (L_IsFounded :type Boolean) (L_EmptySlotsIndexes :type "Array of Integer"))
  (set `local.L_StoreIndex` ToSlot)
  (set `local.L_TemplateIndexes` TemplateIndexes)
  (for _array_element (`local.L_TemplateIndexes`)
    (bind _returnvalue (+ _array_element (`local.L_StoreIndex`)))
    (if (< _returnvalue (`self.NumberOfSlots`))
      (if (== (`.id` (break `DataItems` (`|GetArrayItem` (`self.StoreItems`) _returnvalue))) -1)
        (`KismetArrayLibrary.Array_Add` (`local.L_EmptySlotsIndexes`) _returnvalue)
        (set `local.L_IsFounded` true)
        (else
          (set `local.L_IsFounded` false)
          (break)))
      (else
        (set `local.L_IsFounded` false)
        (break))))
  (return (`local.L_IsFounded`) (`local.L_EmptySlotsIndexes`)))

(fn `CreateItemSlotToInventory`
  (params (TemplateIndexes :type "Array of Integer") (DataItem :type "DataItems Structure"))
  (bind (_id _typeitem _typeequip _name _description _icon _staticmesh _defense _damage _iconsize) (break `DataItems` DataItem))
  (bind _output (`|GetArrayItem` TemplateIndexes))
  (bind _xslots (`self.XSlots`))
  (bind (_column _row) (break `IconSize` _iconsize))
  (bind _returnvalue (`|CreateWidget` "/Game/Stanaris/Hero/UI/W_ItemSlot.W_ItemSlot_C" null _id))
  (bind _returnvalue_2 (`GridPanel.AddChildToGrid` (`/Game/Stanaris/Hero/UI/W_Inventory.GridInventory` (`self.W_InventoryRef`)) _returnvalue))
  (`GridSlot.SetColumn` _returnvalue_2 (mod _output _xslots))
  (`GridSlot.SetRow` _returnvalue_2 (/ _output _xslots))
  (`GridSlot.SetColumnSpan` _returnvalue_2 _column)
  (`GridSlot.SetRowSpan` _returnvalue_2 _row))

(fn `FindEmptySlot`
  (params (IconSize :type "IconSize Structure") (TemplateIndexes :type "Array of Integer"))
  (returns (Found :type Boolean) (EmptySlotsIndex :type "Array of Integer"))
  (locals (L_StoreIndex :type Integer) (L_IsFounded :type Boolean) (L_TemplateIndexes :type "Array of Integer") (L_StoreElement :type "DataItems Structure") (L_EmptySlotsIndexes :type "Array of Integer"))
  (set `local.L_TemplateIndexes` TemplateIndexes)
  (for (_array_element _array_index) (`self.StoreItems`)
    (set `local.L_StoreElement` _array_element)
    (set `local.L_StoreIndex` _array_index)
    (if (`local.L_IsFounded`)
      (break)
      (elif (== (`.id` (break `DataItems` (`local.L_StoreElement`))) -1)
        (bind (_isfounded _emptyslotsindexes) (`self.CanItemToSlots` (`local.L_StoreIndex`) (`local.L_TemplateIndexes`)))
        (set `local.L_IsFounded` _isfounded)
        (set `local.L_EmptySlotsIndexes` _emptyslotsindexes))))
  (return (`local.L_IsFounded`) (`local.L_EmptySlotsIndexes`)))

(fn `InitInventory`
  (set `self.NumberOfSlots` (* (`self.XSlots`) (`self.YSlots`)))
  (`KismetArrayLibrary.Array_Resize` (`self.StoreItems`) (`self.NumberOfSlots`)))

(fn `PlaceItemToStore`
  (params (TemplateIndexes :type "Array of Integer") (Item :type "DataItems Structure (by ref)"))
  (for _array_element TemplateIndexes
    (`KismetArrayLibrary.Array_Set` (`self.StoreItems`) _array_element Item)))