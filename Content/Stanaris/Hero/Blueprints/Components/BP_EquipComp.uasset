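; Hero equipment component that stores equipped items in an array indexed by equipment slot and checks whether slots are empty.
; It builds W_ItemSlot icons from the item table at fixed grid cells per slot type, with two-handed weapons sharing the Weapon cell.
; Equip and unequip set or clear the matching character mesh, then add or subtract stats and refresh the stats widget.
; Character, stats and widget references are injected through setters.
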(fn `CheckEmptySlots`
  (params (SlotsIndex :type "Array of Integer"))
  (returns (Empty :type Boolean))
  (locals (L_IsEmpty :type Boolean :default true))
  (for _array_element SlotsIndex
    (if (not (== (`.id` (break `InventoryItem` (`|GetArrayItem` (`self.EquipItems`) _array_element))) -1))
      (set `local.L_IsEmpty` false)
      (break)))
  (return (`local.L_IsEmpty`)))

(fn `CreateItemSlotToEquip`
  (params (SlotIndex :type Integer) (IdItem :type Integer))
  (locals (L_SlotIndex :type Integer) (L_IdItem :type Integer) (L_TemplateIndexes :type "Array of Integer") (L_Row :type Integer) (L_Column :type Integer) (L_RowSpan :type Integer) (L_ColumnSpan :type Integer) (L_IconSize :type "IconSize Structure") (L_EquipType :type "ETypeEquipment Enum" :default "Other"))
  (bind (_column _row) (break `IconSize` (`local.L_IconSize`)))
  (bind (_success _returnvalue) (`StanarisGameInstanceLibrary.GetItemFromTableById` (`local.L_IdItem`) (`self.ItemsTable`)))
  (bind (_id _typeitem _typeequip _name _description _isstackable _numberonstack _maxnumberonstack _icon _staticmesh _skeletalmesh _defense _damage _iconsize _templateindexes) (break `DataItems` _returnvalue))
  (set `local.L_SlotIndex` SlotIndex)
  (set `local.L_IdItem` IdItem)
  (switch `ETypeEquipment` (cast `ETypeEquipment` (`KismetMathLibrary.Conv_IntToByte` (`local.L_SlotIndex`)))
    (:`Helm`
      (set `local.L_Row` 1)
      (set `local.L_Column` 4)
      (set `local.L_RowSpan` 2)
      (set `local.L_ColumnSpan` 2))
    (:`Neck`
      (set `local.L_Row` 2)
      (set `local.L_Column` 7)
      (set `local.L_RowSpan` 1)
      (set `local.L_ColumnSpan` 1))
    (:`Weapon`
      (set `local.L_Row` 4 :!label _label)
      (set `local.L_Column` 1)
      (set `local.L_RowSpan` 3)
      (set `local.L_ColumnSpan` 2))
    (:`Shield`
      (set `local.L_Row` 4)
      (set `local.L_Column` 7)
      (set `local.L_RowSpan` 3)
      (set `local.L_ColumnSpan` 2))
    (:`RightRing`
      (set `local.L_Row` 8)
      (set `local.L_Column` 1)
      (set `local.L_RowSpan` 1)
      (set `local.L_ColumnSpan` 1))
    (:`LeftRing`
      (set `local.L_Row` 8)
      (set `local.L_Column` 8)
      (set `local.L_RowSpan` 1)
      (set `local.L_ColumnSpan` 1))
    (:`Body`
      (set `local.L_Row` 10)
      (set `local.L_Column` 1)
      (set `local.L_RowSpan` 3)
      (set `local.L_ColumnSpan` 2))
    (:`Pants`
      (set `local.L_Row` 10)
      (set `local.L_Column` 7)
      (set `local.L_RowSpan` 3)
      (set `local.L_ColumnSpan` 2))
    (:`Gloves`
      (set `local.L_Row` 14)
      (set `local.L_Column` 1)
      (set `local.L_RowSpan` 2)
      (set `local.L_ColumnSpan` 2))
    (:`Boots`
      (set `local.L_Row` 14)
      (set `local.L_Column` 7)
      (set `local.L_RowSpan` 2)
      (set `local.L_ColumnSpan` 2))
    (:`Weapon2H`
      (goto _label)))
  (if _success
    (set `local.L_IconSize` _iconsize)
    (set `local.L_TemplateIndexes` _templateindexes)
    (bind _returnvalue_2 (`|CreateWidget` "/Game/Stanaris/Hero/UI/Inventory/W_ItemSlot.W_ItemSlot_C" null (`local.L_IdItem`) (`local.L_SlotIndex`) (`local.L_TemplateIndexes`) "Equip" _typeequip 1))
    (`/Game/Stanaris/Hero/UI/W_Equip.AddItemIcon` (`self.W_EquipRef`) (`local.L_SlotIndex`) _returnvalue_2)
    (bind _returnvalue_3 (`GridPanel.AddChildToGrid` (`self.GridEquipRef`) _returnvalue_2))
    (`GridSlot.SetColumn` _returnvalue_3 (`local.L_Column`))
    (`GridSlot.SetRow` _returnvalue_3 (`local.L_Row`))
    (`GridSlot.SetColumnSpan` _returnvalue_3 (`local.L_ColumnSpan`))
    (`GridSlot.SetRowSpan` _returnvalue_3 (`local.L_RowSpan`))
    (bind _sizeimage (`/Game/Stanaris/Hero/UI/Inventory/W_ItemSlot.SizeImage` _returnvalue_2))
    (`SizeBox.SetWidthOverride` _sizeimage (* _column 50.0))
    (`SizeBox.SetHeightOverride` _sizeimage (* _row 50.0))))

(fn `DeleteDataFromEquipStoreByIndex`
  (params (IndexEquipSlot :type Integer))
  (`KismetArrayLibrary.Array_Set` (`self.EquipItems`) IndexEquipSlot (make `InventoryItem` -1)))

(fn `EquipItem`
  (params (SlotIndexEquip :type Integer) (ItemData :type "DataItems Structure"))
  (locals (L_NewSkeletalMesh :type "SkeletalMesh Object Reference") (L_NewStaticMesh :type "StaticMesh Object Reference") (L_SlotIndexEquip :type Integer) (L_DataItem :type "DataItems Structure"))
  (bind (_id _typeitem _typeequip _name _description _isstackable _numberonstack _maxnumberonstack _icon _staticmesh _skeletalmesh) (break `DataItems` ItemData))
  (bind _characterref (`self.CharacterRef`))
  (set `local.L_SlotIndexEquip` SlotIndexEquip)
  (set `local.L_NewStaticMesh` _staticmesh)
  (set `local.L_NewSkeletalMesh` _skeletalmesh)
  (set `local.L_DataItem` ItemData)
  (switch `ETypeEquipment` (cast `ETypeEquipment` (`KismetMathLibrary.Conv_IntToByte` (`local.L_SlotIndexEquip`)))
    (:`Helm`
      (`/Game/Stanaris/Hero/Blueprints/BP_Character.SetHelm` _characterref (`local.L_NewSkeletalMesh`)))
    (:`Neck`
      (`/Game/Stanaris/Hero/Blueprints/BP_Character.SetNeck` _characterref (`local.L_NewSkeletalMesh`)))
    (:`Weapon`
      (`/Game/Stanaris/Hero/Blueprints/BP_Character.SetRightHand` _characterref (`local.L_NewSkeletalMesh`)))
    (:`Shield`
      (`/Game/Stanaris/Hero/Blueprints/BP_Character.SetLeftHand` _characterref (`local.L_NewSkeletalMesh`)))
    (:`RightRing`
      (`/Game/Stanaris/Hero/Blueprints/BP_Character.SetRightRing` _characterref (`local.L_NewStaticMesh`)))
    (:`LeftRing`
      (`/Game/Stanaris/Hero/Blueprints/BP_Character.SetLeftRing` _characterref (`local.L_NewStaticMesh`)))
    (:`Body`
      (`/Game/Stanaris/Hero/Blueprints/BP_Character.SetBody` _characterref (`local.L_NewSkeletalMesh`)))
    (:`Pants`
      (`/Game/Stanaris/Hero/Blueprints/BP_Character.SetPants` _characterref (`local.L_NewSkeletalMesh`)))
    (:`Gloves`
      (`/Game/Stanaris/Hero/Blueprints/BP_Character.SetGloves` _characterref (`local.L_NewSkeletalMesh`)))
    (:`Boots`
      (`/Game/Stanaris/Hero/Blueprints/BP_Character.SetBoots` _characterref (`local.L_NewSkeletalMesh`)))
    (:`Weapon2H`
      (`/Game/Stanaris/Hero/Blueprints/BP_Character.Set2HRightHand` _characterref (`local.L_NewSkeletalMesh`))))
  (`StatsComp.AddStats` (`self.StatsCompRef`) (`local.L_DataItem`))
  (`/Game/Stanaris/Hero/UI/W_Stats.OnUpdateStats` (`self.W_StatsRef`)))

(fn `PlaceItemToEquipStore`
  (params (IndexEquipSlot :type Integer) (InventoryData :type "InventoryItem Structure (by ref)"))
  (`KismetArrayLibrary.Array_Set` (`self.EquipItems`) IndexEquipSlot InventoryData))

(fn `SetCharacterRef`
  (params (CharacterRef :type "/Game/Stanaris/Hero/Blueprints/BP_Character Object Reference"))
  (set `self.CharacterRef` CharacterRef))

(fn `SetGridEquipRef`
  (params (GridEquip :type "GridPanel Object Reference"))
  (set `self.GridEquipRef` GridEquip))

(fn `SetStatCompRef`
  (params (StatsComp :type "StatsComp Object Reference"))
  (set `self.StatsCompRef` StatsComp))

(fn `SetWEquipRef`
  (params (W_EquipRef :type "/Game/Stanaris/Hero/UI/W_Equip Object Reference"))
  (bind _output_get (set `self.W_EquipRef` W_EquipRef))
  (`self.SetGridEquipRef` (`/Game/Stanaris/Hero/UI/W_Equip.GridEquip` _output_get)))

(fn `SetWStatsRef`
  (params (W_StatsRef :type "/Game/Stanaris/Hero/UI/W_Stats Object Reference"))
  (set `self.W_StatsRef` W_StatsRef))

(fn `UnequipItem`
  (params (SlotIndexType :type Integer) (ItemData :type "DataItems Structure"))
  (locals (L_SlotindexType :type Integer) (L_ItemData :type "DataItems Structure"))
  (bind _characterref (`self.CharacterRef`))
  (set `local.L_SlotindexType` SlotIndexType)
  (set `local.L_ItemData` ItemData)
  (switch `ETypeEquipment` (cast `ETypeEquipment` (`KismetMathLibrary.Conv_IntToByte` (`local.L_SlotindexType`)))
    (:`Helm`
      (`/Game/Stanaris/Hero/Blueprints/BP_Character.SetHelm` _characterref null))
    (:`Neck`
      (`/Game/Stanaris/Hero/Blueprints/BP_Character.SetNeck` _characterref null))
    (:`Weapon`
      (`/Game/Stanaris/Hero/Blueprints/BP_Character.SetRightHand` _characterref null))
    (:`Shield`
      (`/Game/Stanaris/Hero/Blueprints/BP_Character.SetLeftHand` _characterref null))
    (:`RightRing`
      (`/Game/Stanaris/Hero/Blueprints/BP_Character.SetRightRing` _characterref null))
    (:`LeftRing`
      (`/Game/Stanaris/Hero/Blueprints/BP_Character.SetLeftRing` _characterref null))
    (:`Body`
      (`/Game/Stanaris/Hero/Blueprints/BP_Character.SetBody` _characterref null))
    (:`Pants`
      (`/Game/Stanaris/Hero/Blueprints/BP_Character.SetPants` _characterref null))
    (:`Gloves`
      (`/Game/Stanaris/Hero/Blueprints/BP_Character.SetGloves` _characterref null))
    (:`Boots`
      (`/Game/Stanaris/Hero/Blueprints/BP_Character.SetBoots` _characterref null))
    (:`Weapon2H`
      (`/Game/Stanaris/Hero/Blueprints/BP_Character.Set2HRightHand` _characterref null)))
  (`StatsComp.SubtractStats` (`self.StatsCompRef`) (`local.L_ItemData`))
  (`/Game/Stanaris/Hero/UI/W_Stats.OnUpdateStats` (`self.W_StatsRef`)))