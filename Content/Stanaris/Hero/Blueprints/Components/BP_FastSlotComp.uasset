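; BP_FastSlotComp is the hero's quick-slot component, holding items in a fixed number of slots for fast use.
; On BeginPlay it sizes the item store, which place and delete functions write by index.
; CreateItemToFastSlot builds an item-slot widget from items-table data, registers it with the fast panel and lays it out in a single-row grid.
; GetItemForUseByIndex returns a slot's item only if it casts to BP_UsedItem.
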(event `self.ReceiveBeginPlay`
  (`self.Init`))

(fn `CreateItemToFastSlot`
  (params (SlotIndex :type Integer) (IdItem :type Name) (InventoryItem :type "InventoryItem Structure (by ref)") (SizeIcon :type "Float (double-precision)" :default 50.0))
  (locals (L_SlotIndex :type Integer) (L_IdItem :type Name) (L_IconSize :type "IconSize Structure") (L_TemplateIndexes :type "Array of Integer") (L_Column :type Integer) (L_SizeIcon :type "Float (double-precision)" :default 50.0))
  (bind (_column _row) (break `IconSize` (`local.L_IconSize`)))
  (bind (_success _returnvalue) (`StanarisGameInstanceLibrary.GetItemFromTableById` (`local.L_IdItem`) (`self.ItemsTable`)))
  (bind (_id _typeitem _typeequip _name _description _isstackable _numberonstack _maxnumberonstack _icon _staticmesh _skeletalmesh _defense _damage _iconsize _templateindexes) (break `DataItems` _returnvalue))
  (set `local.L_SlotIndex` SlotIndex)
  (set `local.L_IdItem` IdItem)
  (set `local.L_SizeIcon` SizeIcon)
  (if _success
    (set `local.L_IconSize` _iconsize)
    (set `local.L_TemplateIndexes` _templateindexes)
    (bind _returnvalue_2 (`|CreateWidget` "/Game/Stanaris/Hero/UI/Inventory/W_ItemSlot.W_ItemSlot_C" null (`local.L_IdItem`) (`local.L_SlotIndex`) (`local.L_TemplateIndexes`) "FastSlot" _typeequip (`.NumberOfItems` (break `InventoryItem` InventoryItem))))
    (`/Game/Stanaris/Hero/UI/W_FastPanel.AddItemIcon` (`self.W_FastPanel`) (`local.L_SlotIndex`) _returnvalue_2)
    (bind _returnvalue_3 (`GridPanel.AddChildToGrid` (`self.GridEquipRef`) _returnvalue_2))
    (`GridSlot.SetColumn` _returnvalue_3 (`local.L_SlotIndex`))
    (`GridSlot.SetRow` _returnvalue_3 0)
    (`GridSlot.SetColumnSpan` _returnvalue_3 0)
    (`GridSlot.SetRowSpan` _returnvalue_3 0)
    (bind _sizeimage (`/Game/Stanaris/Hero/UI/Inventory/W_ItemSlot.SizeImage` _returnvalue_2))
    (`SizeBox.SetWidthOverride` _sizeimage (* _column (`local.L_SizeIcon`)))
    (`SizeBox.SetHeightOverride` _sizeimage (* _row (`local.L_SizeIcon`)))))

(fn `DeleteFromStore`
  (params (Index :type Integer))
  (`KismetArrayLibrary.Array_Set` (`self.StoreItems`) Index (make `InventoryItem` "none"))
  (return))

(fn `GetItemForUseByIndex`
  (params (IndexStore :type Integer))
  (returns (Success :type Boolean) (UsedItem :type "/Game/Stanaris/Blueprints/Items/Used/BP_UsedItem Object Reference"))
  (bind (_id _numberofitems _typeitem _itemref) (break `InventoryItem` (`|GetArrayItem` (`self.StoreItems`) IndexStore)))
  (if (!= _id "None")
    (bind _asbp_used_item (cast `/Game/Stanaris/Blueprints/Items/Used/BP_UsedItem` _itemref)
      (:`then`
        (return true _asbp_used_item))
      (:`CastFailed`
        _)))
  (return false null))

(fn `Init`
  (`KismetArrayLibrary.Array_Resize` (`self.StoreItems`) (`self.NumberOfSlots`)))

(fn `PlaceItemToStore`
  (params (Index :type Integer) (InventoryItem :type "InventoryItem Structure (by ref)"))
  (`KismetArrayLibrary.Array_Set` (`self.StoreItems`) Index InventoryItem))

(fn `SetFastPanelRef`
  (params (FastPanel :type "/Game/Stanaris/Hero/UI/W_FastPanel Object Reference"))
  (set `self.W_FastPanel` FastPanel))

(fn `SetFastSlotGridRef`
  (params (GridEquipRef :type "GridPanel Object Reference"))
  (set `self.GridEquipRef` GridEquipRef))

(fn `SetInventoryCompRef`
  (params (InventoryCompRef :type "/Game/Stanaris/Hero/Blueprints/Components/BP_InventoryComp Object Reference"))
  (set `self.InventoryCompRef` InventoryCompRef))