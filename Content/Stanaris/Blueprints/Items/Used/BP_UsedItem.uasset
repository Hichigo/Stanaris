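; Consumable item that applies a health effect when used from a fast slot, then updates the slot's count or removes it.
; Use stores the stats component and starts an Instant, Over Time or Temporary effect by type.
; Over Time heals on a looping one-second timer until an end timestamp, destroying the actor if it was the last item.
; Temporary start and end functions are empty stubs, and debug prints remain in the tick.
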(event `self.ReceiveBeginPlay`
  (`parent.ReceiveBeginPlay`))

(fn `InstantEffect`
  (`StatsComp.AddHealth` (`self.StatsCompRef`) 50.0))

(fn `OverTime`
  (`self.OverTimeEffect`)
  (if (>= (`KismetMathLibrary.Now`) (`self.TimeEndTimer`))
    (`KismetSystemLibrary.K2_ClearAndInvalidateTimerHandle` (`self.HandleTimer`))
    (`KismetSystemLibrary.PrintString` "BYE")
    (if (`self.DestroyActor`)
      (`self.K2_DestroyActor` (`self.Actor`)))
    (else
      (`KismetSystemLibrary.PrintString` "Hello"))))

(fn `OverTimeEffect`
  (`StatsComp.AddHealth` (`self.StatsCompRef`) (/ 10.0 (`KismetMathLibrary.Conv_IntToDouble` (`self.Duration`)))))

(fn `StartEffectItem`
  (params (DestroyActor :type Boolean))
  (set `self.DestroyActor` DestroyActor)
  (switch `ETypeEffectUseItem` (`self.TypeEffect`)
    (:`Instant`
      (`self.InstantEffect`))
    (:`OverTime`
      (`self.CreateTimestamp`)
      (bind _returnvalue (`KismetSystemLibrary.K2_SetTimer` null "OverTime" 1.0 true))
      (set `self.HandleTimer` _returnvalue))
    (:`Temporary`
      (`self.CreateTimestamp`)
      (`self.TemporaryEffectStart`)
      (bind _returnvalue_2 (`KismetSystemLibrary.K2_SetTimer` null "TemporaryEffectEnd" (`KismetMathLibrary.Conv_IntToDouble` (`self.Duration`))))
      (set `self.HandleTimer` _returnvalue_2))))

(fn `TemporaryEffectEnd`)

(fn `TemporaryEffectStart`)

(fn `Use`
  (params (FastSlotComp :type "/Game/Stanaris/Hero/Blueprints/Components/BP_FastSlotComp Object Reference") (StatsComp :type "StatsComp Object Reference") (SlotIndex :type Integer))
  (returns (IsLast :type Boolean))
  (locals (L_FastSlotCompRef :type "/Game/Stanaris/Hero/Blueprints/Components/BP_FastSlotComp Object Reference") (L_SlotIndex :type Integer))
  (bind _w_fastpanel (`/Game/Stanaris/Hero/Blueprints/Components/BP_FastSlotComp.W_FastPanel` (`local.L_FastSlotCompRef`)))
  (bind _output (`|GetArrayItem` (`/Game/Stanaris/Hero/Blueprints/Components/BP_FastSlotComp.StoreItems` (`local.L_FastSlotCompRef`)) (`local.L_SlotIndex`)))
  (bind (_id _numberofitems _typeitem _itemref) (break `InventoryItem` _output))
  (bind _value (`BlueprintMapLibrary.Map_Find` (`/Game/Stanaris/Hero/UI/W_FastPanel.WidgetsItem` _w_fastpanel) (`local.L_SlotIndex`)))
  (set `local.L_FastSlotCompRef` FastSlotComp)
  (set `self.StatsCompRef` StatsComp)
  (set `local.L_SlotIndex` SlotIndex)
  (set `self.Actor` _itemref)
  (if (> _numberofitems 1)
    (setmembers `InventoryItem` :`StructRef` _output :`NumberOfItems` (- _numberofitems 1))
    (`self.StartEffectItem` false)
    (`/Game/Stanaris/Hero/UI/Inventory/W_ItemSlot.UpdateNumberOfItems` _value)
    (return false)
    (else
      (`self.StartEffectItem` true)
      (`Widget.RemoveFromParent` _value)
      (`/Game/Stanaris/Hero/UI/W_FastPanel.RemoveItemIcon` _w_fastpanel (`local.L_SlotIndex`))
      (`/Game/Stanaris/Hero/Blueprints/Components/BP_FastSlotComp.DeleteFromStore` (`local.L_FastSlotCompRef`) (`local.L_SlotIndex`))
      (return true))))

(fn `UserConstructionScript`
  (`parent.UserConstructionScript`))