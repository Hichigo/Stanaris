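; BP_BaseItem is the base world item, showing a static mesh from an item table entry chosen by fixed ID or at random.
; The construction script sets the mesh, and BeginPlay resolves the item again, so random items re-roll at play start.
; InitDropOnGround accepts item data directly for drops, SwitchPhysics toggles simulation and collision together, and TouchItem returns the item ID.
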(event `self.ReceiveBeginPlay`
  (if (`self.Random`)
    (`self.InitRandomItem`)
    (else
      (`self.InitItem`))))

(fn `InitDropOnGround`
  (params (IdItem :type Integer) (Data :type "DataItems Structure"))
  (set `self.IdItem` IdItem)
  (bind _output_get (set `self.Data` Data))
  (`StaticMeshComponent.SetStaticMesh` (`self.SM_Item`) (`.StaticMesh` (break `DataItems` _output_get))))

(fn `InitItem`
  (bind (_success _returnvalue) (`StanarisGameInstanceLibrary.GetItemFromTableById` (`self.IdItem`) (`self.ItemsTable`)))
  (if _success
    (set `self.Data` _returnvalue)
    (`StaticMeshComponent.SetStaticMesh` (`self.SM_Item`) (`.StaticMesh` (break `DataItems` (`self.Data`))))))

(fn `InitRandomItem`
  (bind (_success _returnvalue) (`StanarisGameInstanceLibrary.GetItemFromTableById` (`KismetMathLibrary.RandomIntegerInRange` 1 12) (`self.ItemsTable`)))
  (if _success
    (bind _output_get (set `self.Data` _returnvalue))
    (bind (_id _typeitem _typeequip _name _description _isstackable _numberonstack _maxnumberonstack _icon _staticmesh) (break `DataItems` _output_get))
    (`StaticMeshComponent.SetStaticMesh` (`self.SM_Item`) _staticmesh)
    (set `self.IdItem` _id)
    (else
      (`KismetSystemLibrary.PrintString` "INIT RANDOM ERROR"))))

(fn `SwitchPhysics`
  (params (StatePhysics :type Boolean))
  (bind _sm_item (`self.SM_Item`))
  (bind _sm_item_2 (`self.SM_Item`))
  (if StatePhysics
    (`PrimitiveComponent.SetSimulatePhysics` _sm_item true)
    (`PrimitiveComponent.SetCollisionEnabled` _sm_item "QueryAndPhysics")
    (else
      (`PrimitiveComponent.SetSimulatePhysics` _sm_item_2 false)
      (`PrimitiveComponent.SetCollisionEnabled` _sm_item_2 "NoCollision"))))

(fn `TouchItem`
  (returns (IdItem :type Integer))
  (return (`self.IdItem`)))

(fn `UserConstructionScript`
  (locals (L_FoundById :type Boolean :default false))
  (bind (_success _returnvalue) (`StanarisGameInstanceLibrary.GetItemFromTableById` (`self.IdItem`) (`self.ItemsTable`)))
  (if (`self.Random`)
    (`self.InitRandomItem`)
    (elif _success
      (`StaticMeshComponent.SetStaticMesh` (`self.SM_Item`) (`.StaticMesh` (break `DataItems` _returnvalue)))
      (else
        (`KismetSystemLibrary.PrintString` "ITEM NOT FOUND")))))