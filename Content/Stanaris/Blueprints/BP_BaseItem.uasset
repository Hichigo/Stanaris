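; BP_BaseItem is an item actor that takes on a random item definition when play begins.
; BeginPlay picks a random entry from the list returned by GetDataItems, stores it as Data and applies its static mesh to SMItem.
; If that lookup is invalid, it prints a game instance data error instead.
; TouchItem hands the stored Data back to the caller; overlap and tick events are unused.
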(event `self.ReceiveBeginPlay`
  (bind (_isvalid _returnvalue) (`StanarisGameInstanceLibrary.GetDataItems`))
  (if _isvalid
    (bind _output_get (set `self.Data` (`|GetArrayItem` _returnvalue (`KismetMathLibrary.RandomInteger` (`KismetArrayLibrary.Array_Length` _returnvalue)))))
    (`StaticMeshComponent.SetStaticMesh` (`self.SM_Item`) (`.StaticMesh` (break `DataItems` _output_get)))
    (else
      (`KismetSystemLibrary.PrintString` "*** ERROR DATA GAME INSTANCE ***" true true (struct :`R` 1.0 :`A` 1.0) 10.0))))

(fn `TouchItem`
  (returns (DataItem :type "DataItems Structure"))
  (return (`self.Data`)))

(fn `UserConstructionScript`)