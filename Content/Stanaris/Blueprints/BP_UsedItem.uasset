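; BP_UsedItem is a usable item Blueprint that handles consuming one unit of an item from a fast-slot panel.
; Its Use function takes a fast-slot component and index, then decrements a stacked item's count and refreshes its slot widget.
; For the last unit it removes the widget and icon, then returns a destroy flag and item actor reference rather than destroying the actor itself.
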(fn `Use`
  (params (FastSlotComp :type "/Game/Stanaris/Hero/Blueprints/Components/BP_FastSlotComp Object Reference") (Index :type Integer))
  (returns (DestroyActor :type Boolean) (Actor :type "Actor Object Reference"))
  (locals (L_FastSlotCompRef :type "/Game/Stanaris/Hero/Blueprints/Components/BP_FastSlotComp Object Reference") (L_SlotIndex :type Integer :default 0))
  (bind _w_fastpanel (`/Game/Stanaris/Hero/Blueprints/Components/BP_FastSlotComp.W_FastPanel` (`local.L_FastSlotCompRef`)))
  (bind _output (`|GetArrayItem` (`/Game/Stanaris/Hero/Blueprints/Components/BP_FastSlotComp.StoreItems` (`local.L_FastSlotCompRef`)) (`local.L_SlotIndex`)))
  (bind (_id _numberofitems _typeitem _itemref) (break `InventoryItem` _output))
  (bind _value (`BlueprintMapLibrary.Map_Find` (`/Game/Stanaris/Hero/UI/W_FastPanel.WidgetsItem` _w_fastpanel) (`local.L_SlotIndex`)))
  (set `local.L_FastSlotCompRef` FastSlotComp)
  (set `local.L_SlotIndex` Index)
  (if (> _numberofitems 1)
    (setmembers `InventoryItem` :`StructRef` _output :`NumberOfItems` (- _numberofitems 1))
    (`/Game/Stanaris/Hero/UI/Inventory/W_ItemSlot.UpdateNumberOfItems` _value)
    (return false null)
    (else
      (`Widget.RemoveFromParent` _value)
      (`/Game/Stanaris/Hero/UI/W_FastPanel.RemoveItemIcon` _w_fastpanel (`local.L_SlotIndex`))
      (return true _itemref))))

(fn `UserConstructionScript`
  (`parent.UserConstructionScript`))